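; SquareHole is a goal target Blueprint that awards points when a Bullet enters it.
; On a Box overlap it casts the other actor to Bullet and adds that bullet's BulletScore to the Score on the player's BP_ThirdPersonCharacter.
; It then shows GoalLight and hides it after a one-second retriggerable delay, so repeated hits keep the light on.
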(event `self.Box.OnComponentBeginOverlap`
  (params (OverlappedComponent :type "PrimitiveComponent Object Reference") (OtherActor :type "Actor Object Reference") (OtherComp :type "PrimitiveComponent Object Reference") (OtherBodyIndex :type Integer) (bFromSweep :type Boolean) (SweepResult :type "HitResult Structure (by ref)"))
  (bind _asbp_third_person_character (cast `/Game/BluePrints/BP_ThirdPersonCharacter` (`GameplayStatics.GetPlayerPawn` 0) :!pure true))
  (bind _asbullet (cast `/Game/BluePrints/Bullet` OtherActor))
  (set `/Game/BluePrints/BP_ThirdPersonCharacter.score` (+ (`/Game/BluePrints/BP_ThirdPersonCharacter.score` _asbp_third_person_character) (`/Game/BluePrints/Bullet.bulletScore` _asbullet)) _asbp_third_person_character)
  (`SceneComponent.SetVisibility` (`self.GoalLight`) true false)
  (`KismetSystemLibrary.RetriggerableDelay` 1.0)
  (`SceneComponent.SetVisibility` (`self.GoalLight`) false false))

(fn `UserConstructionScript`)